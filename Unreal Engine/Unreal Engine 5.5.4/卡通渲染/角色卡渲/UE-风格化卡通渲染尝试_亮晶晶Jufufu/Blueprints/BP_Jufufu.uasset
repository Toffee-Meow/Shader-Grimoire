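; Character Blueprint for Jufufu that feeds head orientation to toon materials through the MPC_Toon parameter collection.
; Every Tick it reads the world rotation of the head bone (頭) and writes HeadUp, HeadForward and HeadRight as vector parameters.
; The bone axes are remapped: its right vector becomes HeadUp, its up vector HeadForward, and its forward vector HeadRight.
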(event `self.ReceiveTick`
  (params (DeltaSeconds :type "Float (single-precision)"))
  (bind _rotation (.rotation (`SkinnedMeshComponent.GetBoneTransform` (`self.Jufufu`) "頭" "RTS_World")))
  (`KismetMaterialLibrary.SetVectorParameterValue` "/Game/Characters/Jufufu/Material/MPC_Toon.MPC_Toon" "HeadUp" (`KismetMathLibrary.Conv_VectorToLinearColor` (`KismetMathLibrary.GetRightVector` _rotation)))
  (`KismetMaterialLibrary.SetVectorParameterValue` "/Game/Characters/Jufufu/Material/MPC_Toon.MPC_Toon" "HeadForward" (`KismetMathLibrary.Conv_VectorToLinearColor` (`KismetMathLibrary.GetUpVector` _rotation)))
  (`KismetMaterialLibrary.SetVectorParameterValue` "/Game/Characters/Jufufu/Material/MPC_Toon.MPC_Toon" "HeadRight" (`KismetMathLibrary.Conv_VectorToLinearColor` (`KismetMathLibrary.GetForwardVector` _rotation))))

(fn `UserConstructionScript`)