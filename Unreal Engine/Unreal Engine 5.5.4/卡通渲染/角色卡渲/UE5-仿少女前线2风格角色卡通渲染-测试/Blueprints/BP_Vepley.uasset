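; Character Blueprint for Vepley that drives toon face shading from the directional light's angle relative to the head.
; Construction swaps the face material for a dynamic instance and starts a fast looping timer, apparently for UpdateSDFLocation.
; That update takes the first directional light if none is set, derives a signed angular value from dot and cross products against the head socket's forward vector, remaps it through a curve, and writes SDF_Location.
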(event `UpdateSDFLocation`
  (`self.MaterialTarget`
    (:`then`
      (`self.LightTarget`
        (:`then`
          _)
        (:`else`
          (bind _outactors (`GameplayStatics.GetAllActorsOfClass` "/Script/Engine.DirectionalLight"))
          (set `self.LightTarget` (`|GetArrayItem` _outactors))))
      (`MaterialInstanceDynamic.SetScalarParameterValue` (`self.MaterialTarget`) "SDF_Location" (`CurveFloat.GetFloatValue` (`self.SDFCurveMapped`) (`self.Calculate SDF Location`))))
    (:`else`)))

(fn `Calculate SDF Location`
  (returns (`Renturn Value` :type "Float (double-precision)"))
  (bind _returnvalue (`KismetMathLibrary.GetForwardVector` (`self.K2_GetActorRotation` (`self.LightTarget`))))
  (bind _returnvalue_2 (`KismetMathLibrary.GetForwardVector` (`SceneComponent.GetSocketRotation` (`self.Vepley`) (`self.HeadSocketName`))))
  (bind (_returnvalue_x _returnvalue_y _returnvalue_z) (`KismetMathLibrary.BreakVector` (`KismetMathLibrary.Cross_VectorVector` _returnvalue _returnvalue_2)))
  (bind _returnvalue_3 (`KismetMathLibrary.Dot_VectorVector` _returnvalue _returnvalue_2))
  (if (<= _returnvalue_z 0.0)
    (if (<= _returnvalue_3 0.0)
      (return (/ (- -2.0 _returnvalue_3) -2.0))
      (else
        (return (+ (- 1.0 _returnvalue_3) 1.0))))
    (else
      (return (/ _returnvalue_3 -2.0)))))

(fn `UserConstructionScript`
  (bind _facematerial (`self.FaceMaterial`))
  (`|ExecutionSequence`
    (:`then_0`
      (bind _returnvalue (`KismetMaterialLibrary.CreateDynamicMaterialInstance` _facematerial))
      (bind _output_get (set `self.MaterialTarget` _returnvalue))
      (`PrimitiveComponent.SetMaterial` (`self.Vepley`) (`KismetArrayLibrary.Array_Find` (`MeshComponent.GetMaterials` (`self.Vepley`)) _facematerial) _output_get))
    (:`then_1`
      (`KismetSystemLibrary.K2_SetTimerDelegate` (`|CreateDelegate` :!event `UpdateSDFLocation`) 0.01 true))))